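; BP_ViewModelPC is a player controller that demonstrates driving a HUD health display through a view model.
; On BeginPlay it adds WBP_HudScreen to the viewport and caches that widget's HudVM.
; The D and A keys step PlayerHealth up or down within threshold checks, push it via SetHealthValue, and print feedback.
; The controller owns the health value and updates only the view model, never the widget's visuals directly.
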(event `self.ReceiveBeginPlay`
  (bind _returnvalue (`|CreateWidget` "/Game/MVVMPluginExperiment/WBP_HudScreen.WBP_HudScreen_C"))
  (`UserWidget.AddToViewport` _returnvalue 0)
  (bind _viewmodel (`/Game/MVVMPluginExperiment/WBP_HudScreen.GetHudViewModel` _returnvalue))
  (set `self.HudVM` _viewmodel))

(event `Key|D`
  (params (Key :type "Key Structure"))
  (:`Pressed`
    (if (< (`self.PlayerHealth`) 1.0)
      (bind _output_get (set `self.PlayerHealth` (+ (`self.PlayerHealth`) 0.1)))
      (`HudScreenViewModel.SetHealthValue` (`self.HudVM`) _output_get)
      (`KismetSystemLibrary.PrintString` "Health increased!" true true (struct :`R` 0.223109 :`G` 1.0 :`B` 0.470835 :`A` 1.0))
      (else
        (`KismetSystemLibrary.PrintString` "Full health achieved." true true (struct :`G` 1.0 :`B` 0.059509 :`A` 1.0))))))

(event `Key|A`
  (params (Key :type "Key Structure"))
  (:`Pressed`
    (if (> (`self.PlayerHealth`) 0.0)
      (bind _output_get (set `self.PlayerHealth` (- (`self.PlayerHealth`) 0.1)))
      (`HudScreenViewModel.SetHealthValue` (`self.HudVM`) _output_get)
      (`KismetSystemLibrary.PrintString` "Health decreased!" true true (struct :`R` 1.0 :`G` 0.442533 :`B` 0.402712 :`A` 1.0))
      (else
        (`KismetSystemLibrary.PrintString` "You're already dead!" true true (struct :`R` 1.0 :`G` 0.043253 :`A` 1.0))))))

(fn `UserConstructionScript`)